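; Enemy melee attack gameplay ability that plays an attack montage and damages non-friendly players caught by the swing.
; On activation it sets motion warping toward the combat target and picks a random tagged montage from the avatar.
; The montage's gameplay event triggers a small radius check at its combat socket, applying damage and blood effects.
; A hit also fires the MeleeImpact gameplay cue, and the ability ends after the event or montage.
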(event Ability|EventActivateAbility
  (bind _returnvalue (Ability|GetAvatarActorfromActorInfo))
  (bind _returnvalue_2 (Ability|GetAvatarActorfromActorInfo))
  (Variables|Default|SetHasHitTarget false)
  (bind _asenemy_interface (Utilities|Casting|CastToEnemyInterface _returnvalue_2)
    (:then
      (bind _ascombat_interface (Utilities|Casting|CastToCombatInterface _returnvalue_2)
        (:then
          (Class|CombatInterface|SetMotionWarpingTargetLocation _ascombat_interface (Transformation|GetActorLocation (Class|EnemyInterface|GetCombatTarget _asenemy_interface)))
          (Variables|Default|SetTagMontage (Class|AuraDamageGameplayAbility|GetRandomTaggedMontagefromArray (Class|CombatInterface|GetAttackMontages _ascombat_interface)))
          (|PlayMontageandWaitProxy "None" (.Montage (Utilities|Struct|BreakTaggedMontage (Variables|Default|GetTagMontage))) 1.0 "None" false 1.0 0.0 false
            (:then
              (Ability|Tasks|WaitGameplayEvent (.MontageTag (Utilities|Struct|BreakTaggedMontage (Variables|Default|GetTagMontage))) 0
                (:EventReceived
                  (bind _returnvalue_3 (Class|CombatInterface|GetCombatSocketLocation(Message) _returnvalue (.SocketTag (Utilities|Struct|BreakTaggedMontage (Variables|Default|GetTagMontage)))))
                  (Variables|Default|SetCombatSocketLocation _returnvalue_3)
                  (bind _outactors (Class|AuraAbilitySystemLibrary|GetLivePlayerswithRadius _returnvalue (Variables|Default|GetCombatSocketLocation) 45.0 (Utilities|Array|MakeArray _returnvalue)))
                  (for _array_element _outactors
                    (bind _returnvalue_4 (Class|AuraAbilitySystemLibrary|IsNotFriendly (Ability|GetAvatarActorfromActorInfo) _array_element))
                    (if _returnvalue_4
                      (Class|AuraDamageGameplayAbility|CauseDamage _array_element)
                      (Variables|Default|SetHasHitTarget true)
                      (Class|CombatInterface|GetBloodEffectNiagara(Message) _array_element)))
                  (Variables|Default|GetHasHitTarget
                    (:then
                      (bind _returnvalue_5 (Class|EnemyInterface|GetCombatTarget(Message) (Ability|GetAvatarActorfromActorInfo)))
                      (Class|GameplayAbility|ExecuteGameplayCuewithParams "(TagName=\"GameplayCue.MeleeImpact\")" (Ability|GameplayCue|MakeGameplayCueParameters :AggregatedSourceTags (GameplayTags|MakeGameplayTagContainerfromTag (.MontageTag (Utilities|Struct|BreakTaggedMontage (Variables|Default|GetTagMontage)))) :Location (Variables|Default|GetCombatSocketLocation) :EffectCauser (Ability|GetAvatarActorfromActorInfo) :SourceObject _returnvalue_5)))
                    (:else
                      _))
                  (Ability|EndAbility))))
            (:OnCompleted
              (Ability|EndAbility :!label _label))
            (:OnInterrupted
              (goto _label))
            (:OnCancelled
              (goto _label))))
        (:CastFailed
          (Ability|EndAbility :!label _label_2))))
    (:CastFailed
      (goto _label_2))))