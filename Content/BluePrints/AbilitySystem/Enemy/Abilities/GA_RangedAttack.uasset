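; Enemy ranged attack ability that fires a projectile at the avatar's current combat target.
; On activation it sets the motion warping target to that target's location and plays a random tagged montage from the avatar's attack montages.
; It creates a wait for the montage's tag event, but spawns the projectile and ends from that task's immediate Then pin, not on event receipt.
; The montage keeps playing after the ability ends.
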(event Ability|EventActivateAbility
  (bind _returnvalue (Ability|GetAvatarActorfromActorInfo))
  (bind _returnvalue_2 (Class|EnemyInterface|GetCombatTarget(Message) _returnvalue))
  (Class|CombatInterface|SetMotionWarpingTargetLocation(Message) _returnvalue (Transformation|GetActorLocation _returnvalue_2))
  (bind _returnvalue_3 (Class|CombatInterface|GetAttackMontages(Message) _returnvalue))
  (Variables|Default|SetTagmontage (Class|AuraDamageGameplayAbility|GetRandomTaggedMontagefromArray _returnvalue_3))
  (|PlayMontageandWaitProxy "None" (.Montage (Utilities|Struct|BreakTaggedMontage (Variables|Default|GetTagmontage))) 1.0 "None" false 1.0 0.0 false
    (:then
      (Ability|Tasks|WaitGameplayEvent (.MontageTag (Utilities|Struct|BreakTaggedMontage (Variables|Default|GetTagmontage))) 0
        (:then
          (bind _returnvalue_4 (Class|EnemyInterface|GetCombatTarget(Message) _returnvalue))
          (Class|AuraProjectileSpell|SpawnProjectile (Transformation|GetActorLocation _returnvalue_4))
          (Ability|EndAbility))))
    (:OnCompleted
      (Ability|EndAbility :!label _label))
    (:OnInterrupted
      (goto _label))
    (:OnCancelled
      (goto _label))))