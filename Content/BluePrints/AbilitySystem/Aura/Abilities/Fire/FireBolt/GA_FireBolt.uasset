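; GA_FireBolt is a gameplay ability that casts a fire bolt projectile toward the point under the mouse.
; On activation it commits, gets cursor target data and passes the hit location to the avatar's combat interface for motion warping.
; It plays a random tagged attack montage, waits for that montage's gameplay event, then spawns the projectile from its tagged socket.
; The ability ends when the montage completes, blends out, is interrupted or is cancelled.
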(event Ability|EventActivateAbility
  (bind _returnvalue (Ability|GetAvatarActorfromActorInfo))
  (Ability|CommitAbility)
  (bind _tagetdatahandle (|GetTargetDataUnderMouse)
    (:ValidaData
      (Variables|Default|SetProjectileTargetLocation (.Location (Collision|BreakHitResult (Ability|TargetData|GetHitResultfromTargetData _tagetdatahandle))))
      (bind _ascombat_interface (Utilities|Casting|CastToCombatInterface _returnvalue))
      (Class|CombatInterface|SetMotionWarpingTargetLocation _ascombat_interface (Variables|Default|GetProjectileTargetLocation))
      (bind _returnvalue_2 (Class|CombatInterface|GetAttackMontages(Message) _returnvalue))
      (Variables|Default|SetTagmontage (Class|AuraDamageGameplayAbility|GetRandomTaggedMontagefromArray _returnvalue_2))
      (|PlayMontageandWaitProxy "None" (.Montage (Utilities|Struct|BreakTaggedMontage (Variables|Default|GetTagmontage))) 1.0 "None" false 1.0 0.0 false
        (:then
          (Ability|Tasks|WaitGameplayEvent (.MontageTag (Utilities|Struct|BreakTaggedMontage (Variables|Default|GetTagmontage))) 0
            (:EventReceived
              (Class|AuraProjectileSpell|SpawnProjectile (Variables|Default|GetProjectileTargetLocation) (.SocketTag (Utilities|Struct|BreakTaggedMontage (Variables|Default|GetTagmontage))) false 0.0))))
        (:OnCompleted
          (Ability|EndAbility :!label _label))
        (:OnBlendOut
          (goto _label))
        (:OnInterrupted
          (goto _label))
        (:OnCancelled
          (goto _label))))))